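; AI controller for stealth-game enemy NPCs that reacts to noise, chases the player and searches after losing sight.
; On possess it runs the enemy behavior tree and blackboard.
; Perception updates drive a status enum and target keys: noise location, focused player, or last spotted location beyond a minimum distance, also toggling the NPC's Visible flag.
; Death is handled once inside the perception event, playing the animation and changing status.
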(event `self.ReceivePossess`
  (params (PossessedPawn :type "Pawn Object Reference"))
  ;[0.04222 1 0.03125] Standart Settings
  (bind _asbp_character_npc (cast `/Game/StealthGame/Characters/BP_CharacterNPC` PossessedPawn))
  (set `self.NPC` _asbp_character_npc)
  (`self.RunBehaviorTree` "/Game/StealthGame/AI/BehaviorTree_Enemy.BehaviorTree_Enemy")
  (`self.UseBlackboard` "/Game/StealthGame/AI/Blackboard_Enemy.Blackboard_Enemy")
  (bind _output_get (set `self.Status` "NewEnumerator1"))
  (`BlackboardComponent.SetValueAsEnum` (`self.Blackboard`) "Status" _output_get)
  (set `/Game/StealthGame/Characters/BP_CharacterNPC.Visible` false (`self.NPC`)))

(event `self.AIPerception.OnTargetPerceptionUpdated`
  (params (Actor :type "Actor Object Reference") (Stimulus :type "AIStimulus Structure"))
  (set `self.Spotted Actor` Actor)
  (bind _output_get (set `self.Stimulus` Stimulus))
  (if (`/Game/StealthGame/Characters/BP_CharacterNPC.Death` (`self.NPC`))
    ;[0.04222 1 0.03125] Death
    (`/Engine/EditorBlueprintResources/StandardMacros.DoOnce` false
      (:`Completed`
        (`SkeletalMeshComponent.PlayAnimation` (`Character.Mesh` (`self.NPC`)) "/Game/StealthGame/Characters/Animations/Mobility_Pro/In_Place/MOB1_Stand_Relaxed_Death_B_IPC.MOB1_Stand_Relaxed_Death_B_IPC" false)
        (bind _output_get_2 (set `self.Status` "NewEnumerator0"))
        (`BlackboardComponent.SetValueAsEnum` (`self.Blackboard`) "Status" _output_get_2)))
    (else
      (bind (_age _expirationage _strength _stimuluslocation _receiverlocation _tag _bsuccessfullysensed) (break `AIStimulus` _output_get))
      (bind _returnvalue (and (== _tag "Noise") _bsuccessfullysensed))
      ;[0.04222 1 0.03125] Hearing
      (if _returnvalue
        (bind _output_get_3 (set `self.Status` "NewEnumerator4"))
        (`BlackboardComponent.SetValueAsEnum` (`self.Blackboard`) "Status" _output_get_3)
        (`BlackboardComponent.SetValueAsBool` (`self.Blackboard`) "PlayerNoise" _returnvalue)
        (`BlackboardComponent.SetValueAsVector` (`self.Blackboard`) "TargetLocation" _stimuluslocation)
        (if (not (`/Game/StealthGame/Characters/BP_CharacterNPC.Botle` (`self.NPC`)))
          (bind _output_get_4 (set `self.Status` "NewEnumerator1"))
          (`BlackboardComponent.SetValueAsEnum` (`self.Blackboard`) "Status" _output_get_4))
        (elif _bsuccessfullysensed
          ;[0.04222 1 0.03125] Following
          (if (== (`self.Spotted Actor`) (`GameplayStatics.GetPlayerCharacter` 0))
            (`BlackboardComponent.SetValueAsObject` (`self.Blackboard`) "Focused Actor" (`self.Spotted Actor`))
            (bind _output_get_5 (set `self.Status` "NewEnumerator3"))
            (`BlackboardComponent.SetValueAsEnum` (`self.Blackboard`) "Status" _output_get_5)
            (`BlackboardComponent.SetValueAsInt` (`self.Blackboard`) "SearchingIndex" 0)
            (set `/Game/StealthGame/Characters/BP_CharacterNPC.Visible` true (`self.NPC`)))
          (else
            ;[0.04222 1 0.03125] Searching
            (if (>= (`/Game/StealthGame/AI/BP_BPL_GeneralLibrary.Get The Distance` (`self.K2_GetPawn`) (`self.Spotted Actor`)) 200.0)
              (`BlackboardComponent.SetValueAsVector` (`self.Blackboard`) "Last Spotted Location" (`self.K2_GetActorLocation` (`self.Spotted Actor`)))
              (`BlackboardComponent.SetValueAsObject` (`self.Blackboard`) "Focused Actor" null)
              (bind _output_get_6 (set `self.Status` "NewEnumerator2"))
              (`BlackboardComponent.SetValueAsEnum` (`self.Blackboard`) "Status" _output_get_6)
              (set `/Game/StealthGame/Characters/BP_CharacterNPC.Visible` false (`self.NPC`)))))))))

(fn `UserConstructionScript`)