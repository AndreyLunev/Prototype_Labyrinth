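; AI patrolling component for a stealth game that supplies locations along a route of patrol point actors.
; FindNextPoint returns the current point's location and steps the stored index forward or backward for the following call.
; A flip flag reverses direction on reaching the last or first array entry, so the route runs back and forth instead of looping.
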(fn `Find Next Point`
  (returns (Location :type "Vector Structure"))
  (locals (LocalPoint :type "Actor Object Reference"))
  (bind _patrollingpoints (`self.PatrollingPoints`))
  (set `local.LocalPoint` (`|GetArrayItem` (`self.PatrollingPoints`) (`self.Current Point`)))
  ;[0.04222 1 0.03125] Flipping
  (if (`self.Flipped Path`)
    (set `self.Current Point` (- (`self.Current Point`) 1))
    (if (== (`self.Current Point`) (`KismetArrayLibrary.Array_Find` _patrollingpoints (`|GetArrayItem` _patrollingpoints)))
      (set `self.Flipped Path` false)
      (else
        (set `self.Flipped Path` true)))
    (else
      (set `self.Current Point` (+ (`self.Current Point`) 1))
      (if (== (`self.Current Point`) (`KismetArrayLibrary.Array_LastIndex` (`self.PatrollingPoints`)))
        (set `self.Flipped Path` true)
        (else
          (set `self.Flipped Path` false)))))
  (return (`Actor.K2_GetActorLocation` (`local.LocalPoint`))))