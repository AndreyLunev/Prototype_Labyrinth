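; Behavior tree task that picks a random search point near the target's last seen location for stealth AI.
; It reads the last seen location from the Blackboard, finds a random navigable point within a fixed radius around it and writes that to the point location key.
; Each run also increments a searching index on the Blackboard, then finishes with success without checking whether a point was found.
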(event `self.ReceiveExecuteAI`
  (params (OwnerController :type "AIController Object Reference") (ControlledPawn :type "Pawn Object Reference"))
  (`BTFunctionLibrary.SetBlackboardValueAsVector` (`self.Point Location KeySelector`) (`NavigationSystemV1.K2_GetRandomLocationInNavigableRadius` (`BTFunctionLibrary.GetBlackboardValueAsVector` (`self.Last Seen Location KeySelector`)) 300.0 null null))
  (`BTFunctionLibrary.SetBlackboardValueAsInt` (`self.Searching Index KeySelector`) (+ (`BTFunctionLibrary.GetBlackboardValueAsInt` (`self.Searching Index KeySelector`)) 1))
  (`self.FinishExecute` true))