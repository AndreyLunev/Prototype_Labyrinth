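; BP_BotleStand is a bottle stand actor that shows a pickup prompt when the player is in range.
; On begin overlap with BP_Player, it makes the HUD's Pickup element visible unless the player already has a bottle in their pocket.
; On end overlap it hides the prompt; the pickup itself is not handled in this Blueprint.
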(event `self.ReceiveActorBeginOverlap`
  (params (OtherActor :type "Actor Object Reference"))
  (bind _asbp_player (cast `/Game/StealthGame/Characters/BP_Player` OtherActor))
  (if (not (`/Game/StealthGame/Characters/BP_Player.BotleInPocket` _asbp_player))
    (`Widget.SetVisibility` (`/Game/StealthGame/UI/Widget_HUD.Pickup` (`/Game/StealthGame/Characters/BP_Player.HUD` _asbp_player)) "Visible")))

(event `self.ReceiveActorEndOverlap`
  (params (OtherActor :type "Actor Object Reference"))
  (bind _asbp_player (cast `/Game/StealthGame/Characters/BP_Player` OtherActor))
  (`Widget.SetVisibility` (`/Game/StealthGame/UI/Widget_HUD.Pickup` (`/Game/StealthGame/Characters/BP_Player.HUD` _asbp_player)) "Hidden"))

(fn `UserConstructionScript`)