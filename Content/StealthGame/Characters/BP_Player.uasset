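; BP_Player is the stealth game's player character, handling crouching, bottle throwing, music and game over.
; On BeginPlay it creates the HUD widget and plays a music track at its location.
; Crouch lowers walk speed; the Action key picks up a bottle when the HUD prompt shows, or aims and spawns BP_Botle from the hand socket on release.
; Overlapping BP_EndGame pauses the game and reveals the end-screen statistics and buttons.
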(event `self.ReceiveBeginPlay`
  ;[0.04222 1 0.03125] HUD
  (bind _returnvalue (`|CreateWidget` "/Game/StealthGame/UI/Widget_HUD.Widget_HUD_C"))
  (bind _output_get (set `self.HUD` _returnvalue))
  (`UserWidget.AddToViewport` _output_get 0)
  (`GameplayStatics.PlaySoundAtLocation` "/Game/StealthGame/Audio/S_05__IN_THE_ABYSS_57bpm.S_05__IN_THE_ABYSS_57bpm" (`self.K2_GetActorLocation` self) (struct) 1.0 1.0 0.0 null null null))

(event `InputAction|Sit`
  (params (Key :type "Key Structure"))
  ;[0.04222 1 0.03125] Crouch
  (:`Pressed`
    (set `self.Crouching` true)
    (set `CharacterMovementComponent.MaxWalkSpeed` 200.0 (`self.CharacterMovement`)))
  (:`Released`
    (set `self.Crouching` false)
    (set `CharacterMovementComponent.MaxWalkSpeed` 500.0 (`self.CharacterMovement`))))

(event `InputAction|Action`
  (params (Key :type "Key Structure"))
  (bind _hud (`self.HUD`))
  ;[0.04222 1 0.03125] Botle throw
  (:`Pressed`
    (if (`self.BotleInPocket`)
      (set `self.Aim` true)
      (elif (`Widget.IsVisible` (`/Game/StealthGame/UI/Widget_HUD.Pickup` (`self.HUD`)))
        (set `self.BotleInPocket` true)
        (`Widget.SetVisibility` (`/Game/StealthGame/UI/Widget_HUD.Pickup` (`self.HUD`)) "Hidden"))))
  (:`Released`
    (if (and (`self.Aim`) (`self.BotleInPocket`))
      (set `self.BotleInPocket` false)
      (set `self.Aim` false)
      (bind _returnvalue (`|SpawnActorFromClass` "/Game/StealthGame/Actions/BP_Botle.BP_Botle_C" (`KismetMathLibrary.MakeTransform` (`SceneComponent.GetSocketLocation` (`self.Mesh`) "Hand_RSocket") (`self.GetControlRotation`)) "Undefined" "OverrideRootScale" null null))
      (`SceneComponent.K2_AddLocalOffset` (`/Game/StealthGame/Actions/BP_Botle.Destructible` _returnvalue) (600.0 0.0 0.0) false false)
      (set `/Game/StealthGame/UI/Widget_HUD.BotlesDown` (+ (`/Game/StealthGame/UI/Widget_HUD.BotlesDown` _hud) 1) _hud))))

(event `self.ReceiveActorBeginOverlap`
  (params (OtherActor :type "Actor Object Reference"))
  ;[0.04222 1 0.03125] Gameover
  (cast `/Game/StealthGame/Actions/BP_EndGame` OtherActor)
  (`GameplayStatics.SetGamePaused` true)
  (`Widget.SetVisibility` (`/Game/StealthGame/UI/Widget_HUD.Exit` (`self.HUD`)) "Visible")
  (`Widget.SetVisibility` (`/Game/StealthGame/UI/Widget_HUD.TryAgain` (`self.HUD`)) "Visible")
  (`Widget.SetVisibility` (`/Game/StealthGame/UI/Widget_HUD.StatisticB` (`self.HUD`)) "Visible")
  (`Widget.SetVisibility` (`/Game/StealthGame/UI/Widget_HUD.StatisticK` (`self.HUD`)) "Visible")
  (`Widget.SetVisibility` (`/Game/StealthGame/UI/Widget_HUD.Killed` (`self.HUD`)) "Visible")
  (`Widget.SetVisibility` (`/Game/StealthGame/UI/Widget_HUD.Botles` (`self.HUD`)) "Visible")
  (set `PlayerController.bShowMouseCursor` true (`GameplayStatics.GetPlayerController` 0)))

(fn `UserConstructionScript`)