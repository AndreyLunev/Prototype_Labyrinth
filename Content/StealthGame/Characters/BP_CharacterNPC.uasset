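; Guard NPC for a stealth game that can detect the player or be taken down by a bottle.
; Actor overlaps track whether the player is in radius, and Tick turns on the HUD's caught progress while the living guard's Visible flag is also true.
; A bottle overlap while not Visible marks it dead, disables capsule collision and increments the HUD's GuardsDown counter.
; Player leaving hides the progress; Visible is never set in this graph.
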(event `self.ReceiveActorBeginOverlap`
  (params (OtherActor :type "Actor Object Reference"))
  (bind _hud (`/Game/StealthGame/Characters/BP_Player.HUD` (`self.Player`)))
  ;[0.04222 1 0.03125] Check
  (cast `/Game/StealthGame/Actions/BP_Botle` OtherActor
    (:`then`
      (if (not (`self.Visible`))
        (set `self.Death` true)
        (`PrimitiveComponent.SetCollisionEnabled` (`self.CapsuleComponent`) "NoCollision")
        (set `/Game/StealthGame/UI/Widget_HUD.GuardsDown` (+ (`/Game/StealthGame/UI/Widget_HUD.GuardsDown` _hud) 1) _hud)))
    (:`CastFailed`
      (bind _asbp_player (cast `/Game/StealthGame/Characters/BP_Player` OtherActor))
      (set `self.Player` _asbp_player)
      (set `self.InRad` true))))

(event `self.ReceiveActorEndOverlap`
  (params (OtherActor :type "Actor Object Reference"))
  ;[0.04222 1 0.03125] Check
  (bind _asbp_player (cast `/Game/StealthGame/Characters/BP_Player` OtherActor))
  (bind _hud (`/Game/StealthGame/Characters/BP_Player.HUD` _asbp_player))
  (`Widget.SetVisibility` (`/Game/StealthGame/UI/Widget_HUD.CatchedProgress` _hud) "Hidden")
  (set `/Game/StealthGame/UI/Widget_HUD.Catched` false _hud)
  (set `self.InRad` false))

(event `self.ReceiveTick`
  (params (DeltaSeconds :type "Float (single-precision)"))
  (bind _hud (`/Game/StealthGame/Characters/BP_Player.HUD` (`self.Player`)))
  ;[0.04222 1 0.03125] Status Update
  (if (`self.Death`)
    _
    (elif (and (`self.InRad`) (`self.Visible`))
      (`Widget.SetVisibility` (`/Game/StealthGame/UI/Widget_HUD.CatchedProgress` _hud) "Visible")
      (set `/Game/StealthGame/UI/Widget_HUD.Catched` true _hud))))

(fn `UserConstructionScript`)